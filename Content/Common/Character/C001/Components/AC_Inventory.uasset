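; Actor component that holds a character's inventory as an array of game item property structs and handles collecting items.
; CollectGameItem reads the target actor's AC_GameItems component and looks up its name tag through FindExactItem, a linear search of the array.
; On a match, it rewrites the entry with quantity plus one, destroys the actor and prints the new count.
; Items without an existing entry are not added.
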(fn `Collect GameItem`
  (params (`Target Actor` :type "Actor Object Reference"))
  (locals (`Game Items` :type "/Game/Common/GameItems/AC_GameItems Object Reference"))
  (bind _returnvalue (`Actor.GetComponentByClass` `Target Actor` "/Game/Common/GameItems/AC_GameItems.AC_GameItems_C"))
  (if (`KismetSystemLibrary.IsValid` _returnvalue)
    (bind _output_get (set `local.Game Items` _returnvalue))
    (bind (_gameitem_properties_name _gameitem_properties_quantity _gameitem_properties_nametag) (break `/Game/Common/GameItems/F_GameItems_Properties` (`/Game/Common/GameItems/AC_GameItems.GameItem_Properties` _output_get)))
    (bind (_isfound _found_item_index _item_copy) (`self.Find Exact Item` _gameitem_properties_nametag))
    (if _isfound
      (bind (_name _quantity _nametag _describtion _icon _isstackable _istradable _isusable _iscollectable) (break `/Game/Common/GameItems/F_GameItems_Properties` _item_copy))
      (`KismetArrayLibrary.Array_Set` (`self.GameItems`) _found_item_index (make `/Game/Common/GameItems/F_GameItems_Properties` _name (+ _quantity 1) _nametag _describtion _icon _isstackable _istradable _isusable _iscollectable))
      (`Actor.K2_DestroyActor` (`local.Target Actor`))
      (bind (_output_name _output_quantity) (break `/Game/Common/GameItems/F_GameItems_Properties` (`|GetArrayItem` (`self.GameItems`) _found_item_index)))
      (`KismetSystemLibrary.PrintString` (`KismetStringLibrary.Conv_IntToString` _output_quantity)))))

(fn `Find Exact Item`
  (params (`Target Name Tag` :type "GameplayTag Structure"))
  (returns (isFound :type Boolean) (`Found Item Index` :type Integer) (`Item Copy` :type "/Game/Common/GameItems/F_GameItems_Properties Structure"))
  (locals (Found :type Boolean) (`item index` :type Integer))
  (for (_array_element _array_index) (`self.GameItems`)
    (if (== (`.nametag_21_5F98E1D049FC8EE98DA88B8DD0F418F1` (break `/Game/Common/GameItems/F_GameItems_Properties` _array_element)) (`local.Target Name Tag`))
      (set `local.Found` true)
      (set `local.item index` _array_index)
      (break)))
  (return (`local.Found`) (`local.item index`) (`|GetArrayItem` (`self.GameItems`) (`local.item index`))))