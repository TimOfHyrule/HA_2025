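; AC_Stats is a character component that tracks HP, humidity and movement speed values.
; HP and humidity edits clamp or reset the values and message the owner when HP empties or humidity hits zero or maximum.
; A separate function averages humidity toward its base.
; Stacking speed modifiers scale base speed within a clamped multiplier, with boosts cleared by a five-second timer; HP and speed changes print to screen.
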(event `increase speed`
  (`self.Edit Speed Modifier` 1)
  (`self.Speed Update`)
  (`KismetSystemLibrary.K2_SetTimerDelegate` (delegate `Reset Speed`) 5.0))

(event `Reset Speed`
  (set `self.Modifier Count` 0)
  (`self.Speed Update`))

(fn `Edit HP`
  (params (`Change Amount` :type Integer) (Reset :type Boolean))
  (`|ExecutionSequence`
    (:`then_0`
      (if Reset
        (set `self.HP Current` (`self.HP Base`))
        (else
          (set `self.HP Current` (`KismetMathLibrary.FClamp` (+ (`self.HP Current`) `Change Amount`) 0.0 (`self.HP Max`))))))
    (:`then_1`
      (if (== (`self.HP Current`) 0.0)
        (message `/Game/Common/Character/BPI_Stats.on hp reach 0` (`self.GetOwner`))))
    (:`then_2`
      (`KismetSystemLibrary.PrintString` (`KismetStringLibrary.Conv_DoubleToString` (`self.HP Current`))))))

(fn `Edit Humi Toward Base`
  (set `self.Humidity Current` (/ (+ (`self.Humidity Base`) (`self.Humidity Current`)) 2.0)))

(fn `Edit Humidity`
  (params (`Change Amount` :type "Float (double-precision)") (Reset :type Boolean))
  (bind _returnvalue (`self.GetOwner`))
  (`|ExecutionSequence`
    (:`then_0`
      (if Reset
        (set `self.Humidity Current` (`self.Humidity Base`))
        (else
          (set `self.Humidity Current` (`KismetMathLibrary.FClamp` (+ (`self.Humidity Current`) `Change Amount`) 0.0 (`self.Humidity Max`))))))
    (:`then_1`
      (if (== (`self.Humidity Current`) 0.0)
        (message `/Game/Common/Character/BPI_Stats.on humidity reach 0` _returnvalue)
        (elif (== (`self.Humidity Current`) (`self.Humidity Max`))
          (message `/Game/Common/Character/BPI_Stats.on humidity reach max` _returnvalue))))))

(fn `Edit Speed Modifier`
  (params (`Amount (10%)` :type Integer))
  (locals (`total modifier` :type "Float (double-precision)" :default 1.0))
  (set `self.Modifier Count` (+ `Amount (10%)` (`self.Modifier Count`))))

(fn `Speed Update`
  (bind _output_get (set `self.Speed Current` (* (`KismetMathLibrary.FClamp` (+ (* (`self.Modifier Count`) (`self.Speed Modifier `)) 1.0) 0.5 2.0) (`self.Speed Base`))))
  (`KismetSystemLibrary.PrintString` (`KismetStringLibrary.Conv_DoubleToString` _output_get)))