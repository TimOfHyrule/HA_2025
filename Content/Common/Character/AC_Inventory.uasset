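; Inventory component that tracks item quantities by tag for collecting, buying with coins, quest rewards, dropping and giving items to the player.
; EditItemQuantity is the central update, changing only entries already in the GameItems array, then refreshing the third-person character's inventory UI.
; UseSelectedItem dispatches on the selected tag: Juicy Fruit restores humidity and HP, while Seaweed and Flower only print messages.
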(event `self.ReceiveBeginPlay`
  (`self.Select Item` (struct :`TagName` "NameTag.GameItems.A001_JuicyFruit"))
  (bind _asbp_third_person_character (cast `/Game/ThirdPerson/Blueprints/BP_ThirdPersonCharacter` (`self.GetOwner` self)))
  (bind _output_get (set `self.As BP Third Person Character` _asbp_third_person_character))
  (set `self.Inventory UI` (`/Game/ThirdPerson/Blueprints/BP_ThirdPersonCharacter.inventory UI` _output_get)))

(fn `Collect GameItem`
  (params (`Target Actor` :type "Actor Object Reference"))
  (returns (success :type Boolean))
  (locals (`Game Items component` :type "/Game/Common/GameItems/AC_GameItems Object Reference") (`game item` :type "Actor Object Reference"))
  (bind _returnvalue (`Actor.GetComponentByClass` `Target Actor` "/Game/Common/GameItems/AC_GameItems.AC_GameItems_C"))
  (set `local.game item` `Target Actor`)
  (if (`KismetSystemLibrary.IsValid` _returnvalue)
    (bind _output_get (set `local.Game Items component` _returnvalue))
    (bind (_gameitem_properties_name _gameitem_properties_quantity _gameitem_properties_nametag _gameitem_properties_describtion _gameitem_properties_icon _gameitem_properties_actor _gameitem_properties_isstackable _gameitem_properties_istradable _gameitem_properties_isusable _gameitem_properties_iscollectable _gameitem_properties_isforsell) (break `/Game/Common/GameItems/F_GameItems_Properties` (`/Game/Common/GameItems/AC_GameItems.GameItem_Properties` _output_get)))
    (if _gameitem_properties_isforsell
      (return false)
      (else
        (`self.Edit Item Quantity` _gameitem_properties_nametag 1)
        (`Actor.K2_DestroyActor` (`local.game item`))
        (return true)))))

(fn `Edit Item Quantity`
  (params (`Name Tag` :type "GameplayTag Structure") (`Changed Amount` :type Integer))
  (locals (`item index` :type Integer :default 2) (`item name` :type Text))
  (`|ExecutionSequence`
    (:`then_0`
      (bind (_isfound _found_item_index) (`self.Find Exact Item` `Name Tag`))
      (set `local.item index` _found_item_index)
      (if _isfound
        (bind (_output_name _output_quantity _output_nametag _output_describtion _output_icon _output_actor _output_isstackable _output_istradable _output_isusable _output_iscollectable) (break `/Game/Common/GameItems/F_GameItems_Properties` (`|GetArrayItem` (`self.GameItems`) _found_item_index)))
        (`KismetArrayLibrary.Array_Set` (`self.GameItems`) _found_item_index (make `/Game/Common/GameItems/F_GameItems_Properties` _output_name (+ `Changed Amount` _output_quantity) _output_nametag _output_describtion _output_icon _output_actor _output_isstackable _output_istradable _output_isusable _output_iscollectable))
        (set `local.item name` _output_name)
        (if (== (`self.Selected Item Index`) _found_item_index)
          (set `self.Selected Item` (`|GetArrayItem` (`self.GameItems`) (`local.item index`))))
        (else
          (`KismetSystemLibrary.PrintString` "item not found"))))
    (:`then_1`
      (`/Game/Common/UI/InventoryUI/WI_Inventory.Update Item UI` (`/Game/ThirdPerson/Blueprints/BP_ThirdPersonCharacter.inventory UI` (`self.As BP Third Person Character`)) (`local.item index`))
      (`KismetSystemLibrary.PrintString` (`KismetSystemLibrary.MakeLiteralString` (`KismetStringLibrary.Concat_StrStr` (`KismetTextLibrary.Conv_TextToString` (`local.item name`)) "   " (`KismetStringLibrary.Conv_IntToString` (`local.Changed Amount`)))) true true (struct :`G` 0.66 :`B` 1.0 :`A` 1.0) 10.0))))

(fn `Find Exact Item`
  (params (`Target Name Tag` :type "GameplayTag Structure"))
  (returns (isFound :type Boolean) (`Found Item Index` :type Integer) (`Item Copy` :type "/Game/Common/GameItems/F_GameItems_Properties Structure"))
  (locals (Found :type Boolean) (`item index` :type Integer))
  (for (_array_element _array_index) (`self.GameItems`)
    (if (== (`.nametag_21_5F98E1D049FC8EE98DA88B8DD0F418F1` (break `/Game/Common/GameItems/F_GameItems_Properties` _array_element)) (`local.Target Name Tag`))
      (set `local.Found` true)
      (set `local.item index` _array_index)
      (break)))
  (return (`local.Found`) (`local.item index`) (`|GetArrayItem` (`self.GameItems`) (`local.item index`))))

(fn `Has Amount`
  (params (`Name Tag` :type "GameplayTag Structure") (Amount :type Integer))
  (returns (Result :type Boolean))
  (bind (_isfound _found_item_index _item_copy) (`self.Find Exact Item` `Name Tag`))
  (if _isfound
    (return (>= (`.quantity_22_B31A577C47614FF901EDDABDE0F2A3C8` (break `/Game/Common/GameItems/F_GameItems_Properties` _item_copy)) Amount))))

(fn `Owner Drops Items`
  (bind _returnvalue_location (`KismetMathLibrary.BreakTransform` (`Actor.GetTransform` (`self.GetOwner`))))
  (for _array_element (`self.GameItems`)
    (bind (_name _quantity _nametag _describtion _icon _actor) (break `/Game/Common/GameItems/F_GameItems_Properties` _array_element))
    (for _ (range 1 (+ _quantity 1))
      (`|SpawnActorFromClass` _actor (`KismetMathLibrary.MakeTransform` _returnvalue_location) "Undefined" "MultiplyWithRoot" null null))))

(fn `Owner Gives Player Items`
  (params (`Item Name Tags` :type "Array of GameplayTag Structure") (Amount :type "Array of Integer"))
  (for (_array_element _array_index) `Item Name Tags`
    (`self.Edit Item Quantity` (`Actor.GetComponentByClass` (`GameplayStatics.GetPlayerCharacter` 0) "AC_Inventory_C") _array_element (`|GetArrayItem` Amount _array_index))))

(fn `Quest Reward`
  (params (`Reward Info` :type "/Game/Common/Character/Quest/Struct_RewardInfo Structure"))
  (bind (_itemtag _quantity) (break `/Game/Common/Character/Quest/Struct_RewardInfo` `Reward Info`))
  (for (_array_element _array_index) _itemtag
    (`self.Edit Item Quantity` _array_element (`|GetArrayItem` _quantity _array_index))))

(fn `Select Item`
  (params (`Target Name Tag` :type "GameplayTag Structure"))
  (bind (_isfound _found_item_index _item_copy) (`self.Find Exact Item` `Target Name Tag`))
  (set `self.Selected Item` _item_copy)
  (set `self.Selected Item Index` _found_item_index)
  (`/Engine/EditorBlueprintResources/StandardMacros.IsValid` (`self.Inventory UI`)
    (:`Is Valid`
      (`/Game/Common/UI/InventoryUI/WI_Inventory.Update Select Item UI` (`self.Inventory UI`)))))

(fn `Try Buy GameItem`
  (params (`game item` :type "Actor Object Reference"))
  (bind _returnvalue (`Actor.GetComponentByClass` `game item` "/Game/Common/GameItems/AC_GameItems.AC_GameItems_C"))
  (set `self.game item` `game item`)
  (if (`KismetSystemLibrary.IsValid` _returnvalue)
    (bind _output_get (set `self.Game Items component` _returnvalue))
    (bind (_gameitem_properties_name _gameitem_properties_quantity _gameitem_properties_nametag _gameitem_properties_describtion _gameitem_properties_icon _gameitem_properties_actor _gameitem_properties_isstackable _gameitem_properties_istradable _gameitem_properties_isusable _gameitem_properties_iscollectable _gameitem_properties_isforsell _gameitem_properties_price) (break `/Game/Common/GameItems/F_GameItems_Properties` (`/Game/Common/GameItems/AC_GameItems.GameItem_Properties` _output_get)))
    (if _gameitem_properties_isforsell
      (bind _result (`self.Has Amount` (struct :`TagName` "NameTag.GameItems.A007_Coin") _gameitem_properties_price))
      (if _result
        (`self.Edit Item Quantity` (struct :`TagName` "NameTag.GameItems.A007_Coin") (* _gameitem_properties_price -1))
        (`self.Edit Item Quantity` _gameitem_properties_nametag _gameitem_properties_quantity)
        (`Actor.K2_DestroyActor` (`local.game item`))
        (`KismetSystemLibrary.PrintString` "Sold!")
        (else
          (`KismetSystemLibrary.PrintString` "Not Enough Coins"))))))

(fn `Use A001 Juicy Fruit`
  (bind _ac_stats (`/Game/ThirdPerson/Blueprints/BP_ThirdPersonCharacter.AC_Stats` (`self.As BP Third Person Character`)))
  (bind _result (`self.Has Amount` (struct :`TagName` "NameTag.GameItems.A001_JuicyFruit") 1))
  (if _result
    (`self.Edit Item Quantity` (struct :`TagName` "NameTag.GameItems.A001_JuicyFruit") -1)
    (`/Game/Common/Character/AC_Stats.Edit Humidity` _ac_stats 10.0 false)
    (`/Game/Common/Character/AC_Stats.Edit HP` _ac_stats 20 false)
    (else
      (`KismetSystemLibrary.PrintString` "Not Enough Fruit"))))

(fn `Use A005 Seaweed`
  (`KismetSystemLibrary.PrintString` "USE Seaweed"))

(fn `Use A006 Flower`
  (`KismetSystemLibrary.PrintString` "USE flower"))

(fn `Use Selected Item`
  (bind (_selected_item_name _selected_item_quantity _selected_item_nametag) (break `/Game/Common/GameItems/F_GameItems_Properties` (`self.Selected Item`)))
  (`|ExecutionSequence`
    (:`then_0`
      (if (== _selected_item_nametag (struct :`TagName` "NameTag.GameItems.A001_JuicyFruit"))
        (`self.Use A001 Juicy Fruit`)))
    (:`then_1`
      (if (== _selected_item_nametag (struct :`TagName` "NameTag.GameItems.A005_Seaweed"))
        (`self.Use A005 Seaweed`)))
    (:`then_2`
      (if (== _selected_item_nametag (struct :`TagName` "NameTag.GameItems.A006_Flower"))
        (`self.Use A006 Flower`)))))