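; Quest-giver component that tracks progress through an ordered quest list and sets the dialogue context from the selected action.
; On Finish it asks the owner whether conditions are met, then marks the current quest finished and grants its reward through the player's AC_Inventory.
; Separate functions advance the quest index and derive the sequence state from that index, the list bounds and the finished flag.
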(event `self.ReceiveBeginPlay`
  (set `self.owner` (`self.GetOwner`)))

(fn `Activate Next Quest`
  (set `self.Current Quest Tracker` (+ (`self.Current Quest Tracker`) 1)))

(fn `Update Dialogue Conext`
  (params (`Action Selection` :type "/Game/Common/Character/Quest/Enum_QuestAction Enum" :default "NewEnumerator0"))
  (bind _quest_info (`self.Quest Info`))
  (bind _current_quest_tracker (`self.Current Quest Tracker`))
  (bind (_output_questtag _output_name _output_describtion _output_instruction) (break `/Game/Common/Character/Quest/Struct_QuestInfo` (`|GetArrayItem` _quest_info _current_quest_tracker)))
  (switch `/Game/Common/Character/Quest/Enum_QuestAction` `Action Selection`
    (:`NewEnumerator1`
      (set `self.Dialogue Context` "NewEnumerator1"))
    (:`NewEnumerator2`
      (set `self.Dialogue Context` "NewEnumerator2"))
    (:`NewEnumerator3`
      (bind _result (message `/Game/Common/Character/Quest/BPI_Quest.Quest Finish Condition Check` (`self.owner`) (`self.Current Quest Tracker`)))
      (if _result
        (set `self.Dialogue Context` "NewEnumerator3")
        (`KismetArrayLibrary.Array_Set` _quest_info _current_quest_tracker (make `/Game/Common/Character/Quest/Struct_QuestInfo` _output_questtag _output_name _output_describtion _output_instruction true))
        (`/Game/Common/Character/AC_Inventory.Quest Reward` (`Actor.GetComponentByClass` (`GameplayStatics.GetPlayerCharacter` 0) "/Game/Common/Character/AC_Inventory.AC_Inventory_C") (`|GetArrayItem` (`self.Reward Info`) (`self.Current Quest Tracker`)))
        (else
          (set `self.Dialogue Context` "NewEnumerator4"))))
    (:`NewEnumerator4`
      (set `self.Dialogue Context` "NewEnumerator5"))))

(fn `Update Quest Sequence State`
  (bind _returnvalue (`KismetArrayLibrary.Array_IsValidIndex` (`self.Quest Info`) (+ (`self.Current Quest Tracker`) 1)))
  (if (`KismetArrayLibrary.Array_IsEmpty` (`self.Quest Info`))
    (set `self.Quest Sequence State` "NewEnumerator0")
    (elif (== (`self.Current Quest Tracker`) -1)
      (set `self.Quest Sequence State` "NewEnumerator1")
      (elif (and (not _returnvalue) (`.Finished_14_1C92EB95419FB0A5FD94DAB9B2578C6B` (break `/Game/Common/Character/Quest/Struct_QuestInfo` (`|GetArrayItem` (`self.Quest Info`) (`self.Current Quest Tracker`)))))
        (set `self.Quest Sequence State` "NewEnumerator3")
        (elif _returnvalue
          (set `self.Quest Sequence State` "NewEnumerator1")
          (else
            (set `self.Quest Sequence State` "NewEnumerator2")))))))