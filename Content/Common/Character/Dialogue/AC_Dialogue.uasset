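; Actor component that stores a list of dialogues and hands out the next active dialogue chain on request.
; GetCurrentDialogue first advances the current index, then returns that entry's DialogueChain, so repeated calls cycle through the active entries.
; The advance picks the first active entry after the current index, otherwise falls back to the first active one, leaving the index unchanged if none are active.
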(fn `Get Current Dialogue`
  (returns (`dialogue chain` :type "Array of Text"))
  (`self.Go To Next Avaliavle Index`)
  (return (`.dialoguechain_30_F615383A478112F09E274785A76F6DF5` (break `/Game/Common/Character/Dialogue/Struct_DialogueChain` (`|GetArrayItem` (`self.Dialogue Lists`) (`self.Current Dialogue Index`))))))

(fn `Go To Next Avaliavle Index`
  (locals (`temp index` :type Integer) (found :type Boolean))
  (for (_array_element _array_index) (`self.Dialogue Lists`)
    (if (and (`.isactive_26_E44350F9459DFD9A774FBBADDAFCD298` (break `/Game/Common/Character/Dialogue/Struct_DialogueChain` _array_element)) (> _array_index (`self.Current Dialogue Index`)))
      (set `self.Current Dialogue Index` _array_index)
      (set `local.found` true)
      (break)))
  (if (not (`local.found`))
    (for (_array_element_2 _array_index_2) (`self.Dialogue Lists`)
      (if (`.isactive_26_E44350F9459DFD9A774FBBADDAFCD298` (break `/Game/Common/Character/Dialogue/Struct_DialogueChain` _array_element_2))
        (set `self.Current Dialogue Index` _array_index_2)
        (break)))))